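; BP_Door_01 is an interactable door that swings open and closed on alternate OnInteract calls.
; A FlipFlop plays or reverses the Door timeline, which drives the yaw of SDoor's relative rotation.
; Two DoOnce nodes reset each other to alternate the open and close sounds, both played at world origin rather than the door's location.
; Any actor beginning overlap with the door stops the timeline mid-swing.
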(event EventOnInteract
  ;[1 1 1] Open Door
  (Utilities|FlowControl|FlipFlop
    (:A
      (Utilities|FlowControl|Sequence
        (:then_0
          (Utilities|FlowControl|DoOnce false :!label _label
            (:Completed
              (Audio|PlaySoundatLocation "/Game/VictorianPorps/S_OpenDoor_01.S_OpenDoor_01" "0, 0, 0" "0, 0, 0" 1.0 1.0 0.0 0 0 0 0)
              (goto _label_2 Reset))))
        (:then_1
          (bind _doorrotater (Timeline|Door Play)
            (:Update
              (Transformation|SetRelativeRotation (Variables|Default|GetS_Door) (Math|Rotator|MakeRotator 0.0 0.0 _doorrotater) false false))))))
    (:B
      (Utilities|FlowControl|Sequence
        (:then_0
          (Timeline|Door Reverse))
        (:then_1
          (Utilities|FlowControl|DoOnce false :!label _label_2
            (:Completed
              (Audio|PlaySoundatLocation "/Game/VictorianPorps/S_CloseDoor_01.S_CloseDoor_01" "0, 0, 0" "0, 0, 0" 1.0 1.0 0.0 0 0 0 0)
              (goto _label Reset))))))))

(event Collision|EventActorBeginOverlap
  (params (OtherActor :type Actor%20Object%20Reference))
  ;[1 1 1] Open Door
  (bind _doorrotater (Timeline|Door Stop)
    (:Update
      (Transformation|SetRelativeRotation (Variables|Default|GetS_Door) (Math|Rotator|MakeRotator 0.0 0.0 _doorrotater) false false))))

(fn ConstructionScript)